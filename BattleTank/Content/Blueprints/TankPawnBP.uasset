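; TankPawnBP is the tank pawn Blueprint, and its graphs handle the player's aim rotation.
; The AimAzimuth axis yaws AimGimbal and AimElevation pitches SpringArm, each scaled by delta seconds and its own scale variable.
; It uses AddRelativeRotation for better feel, leaving AddLocalRotation alternatives unconnected.
; BeginPlay, overlap, Tick and the construction script contain no logic.
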(event `InputAxis|AimAzimuth`
  (params (AxisValue :type "Float (single-precision)"))
  ;[1 1 1] Aim Rotation Controls ... Lesson calls for AddLocalRotation but AddRelativeRotation has better feel IMO
  (`SceneComponent.K2_AddRelativeRotation` (`self.AimGimbal`) (`KismetMathLibrary.MakeRotator` 0.0 0.0 (* AxisValue (`GameplayStatics.GetWorldDeltaSeconds`) (`self.AimAzimuthScale`))) false false))

(event `InputAxis|AimElevation`
  (params (AxisValue :type "Float (single-precision)"))
  ;[1 1 1] Aim Rotation Controls ... Lesson calls for AddLocalRotation but AddRelativeRotation has better feel IMO
  (`SceneComponent.K2_AddRelativeRotation` (`self.SpringArm`) (`KismetMathLibrary.MakeRotator` 0.0 (* AxisValue (`GameplayStatics.GetWorldDeltaSeconds`) (`self.AimElevationScale`))) false false))

(fn `UserConstructionScript`)